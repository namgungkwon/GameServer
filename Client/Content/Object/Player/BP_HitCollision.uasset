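; BP_HitCollision is a player-side sphere collision actor that tracks the monsters inside its area.
; Overlap begin and end events cast the other actor to BP_Monster and add it uniquely to, or remove it from, a Targets array.
; GetTargets exposes that array, and SetRaduis resizes the sphere and updates overlaps immediately.
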(event EventBeginPlay)

(event Collision|EventActorBeginOverlap
  (params (OtherActor :type Actor%20Object%20Reference))
  (bind _asbp_monster (Utilities|Casting|CastToBP_Monster OtherActor))
  (Utilities|Array|AddUnique (Variables|Default|GetTargets) _asbp_monster))

(event Collision|EventActorEndOverlap
  (params (OtherActor :type Actor%20Object%20Reference))
  (bind _asbp_monster (Utilities|Casting|CastToBP_Monster OtherActor))
  (Utilities|Array|RemoveItem (Variables|Default|GetTargets) _asbp_monster))

(fn ConstructionScript)

(fn GetTargets
  (return (Variables|Default|GetTargets)))

(fn SetRaduis
  (params (raduis :type Float%20%28double-precision%29))
  (Components|Sphere|SetSphereRadius (Variables|Default|GetSphere) raduis true))