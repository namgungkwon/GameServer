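; Locally controlled player character Blueprint for a networked game, linking packet-driven events to the main HUD, chat and death screen.
; Spawn and update events push HP, MP, EXP and level to UI_Main, while Enter, Tab and mouse wheel drive its chat.
; Attack input, gated by a delay, sets the animation flag, spawns a short-lived BP_HitCollision to gather targets and sends them in an attack packet.
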(event Custom|커스텀이벤트
  (Actor|DestroyActor (stale EventAttackInputPressed _returnvalue)))

(event EventBeginPlay
  (bind _returnvalue (UserInterface|CreateWidget "/Game/Object/UI_Main.UI_Main_C"))
  (bind _output_get (Variables|Default|SetMainWidget _returnvalue))
  (UserInterface|Viewport|AddtoViewport _output_get 0))

(event Collision|EventActorBeginOverlap
  (params (OtherActor :type Actor%20Object%20Reference)))

(event EventTick
  (params (DeltaSeconds :type Float%20%28single-precision%29)))

(event EventSpawnPktReceived
  (bind _mainwidget (Variables|Default|GetMainWidget))
  (Default|SetHp _mainwidget (Variables|Default|GetHp) (Variables|Default|GetMaxHp))
  (Default|SetMp _mainwidget (Variables|Default|GetMp) (Variables|Default|GetMaxMp))
  (Default|SetExp _mainwidget (Variables|Default|GetExp) (Variables|Default|GetRequiredExp))
  (Default|SetName _mainwidget (Variables|Default|GetName))
  (Default|SetLevel _mainwidget (Variables|Default|GetLevel)))

(event EventAttackInputPressed
  (if (not (> (Variables|Default|Getattackdelay) 0.0))
    (Variables|Default|Setmovedelay (* (Variables|Default|GetCONST_MOVE_DELAY) 1.1))
    (Variables|Default|Setattackdelay (Variables|Default|GetCONST_ATTACK_DELAY))
    (Variables|Default|Setabp_isAttack true)
    (bind _returnvalue (Game|SpawnActorfromClass "/Game/Object/Player/BP_HitCollision.BP_HitCollision_C" (Transformation|GetActorTransform) "Undefined" "MultiplyWithRoot" 0 0))
    (Default|SetRaduis _returnvalue 2e+02)
    (bind _targets (Default|GetTargets _returnvalue))
    (Class|MyPlayer|SendAttackPkt _targets)
    (Utilities|Time|SetTimerbyEvent (delegate Custom|커스텀이벤트) 0.3)))

(event EventChatReceived
  (Default|AddChatMessage (Variables|Default|GetMainWidget) (Variables|Default|GetSender) (Variables|Default|GetMessage)))

(event EventDead
  (bind _self self)
  (bind _as플레이어_컨트롤러 (Utilities|Casting|CastToPlayerController (Pawn|GetController _self)))
  (bind _returnvalue (UserInterface|CreateWidget "/Game/Object/BP_DeadWidget.BP_DeadWidget_C" _as플레이어_컨트롤러))
  (Default|SetOwner _returnvalue _self)
  (UserInterface|Viewport|AddtoViewport _returnvalue 0))

(event EventUIUpdate
  (bind _mainwidget (Variables|Default|GetMainWidget))
  (Default|SetHp _mainwidget (Variables|Default|GetHp) (Variables|Default|GetMaxHp))
  (Default|SetMp _mainwidget (Variables|Default|GetMp) (Variables|Default|GetMaxMp))
  (Default|SetExp _mainwidget (Variables|Default|GetExp) (Variables|Default|GetRequiredExp))
  (Default|SetLevel _mainwidget (Variables|Default|GetLevel)))

(event Input|KeyboardEvents|Enter
  (params (Key :type Key%20Structure :default "None"))
  (:Pressed
    (Default|FocusChat (Variables|Default|GetMainWidget))))

(event Input|MouseEvents|MouseWheelUp
  (params (Key :type Key%20Structure :default "None"))
  (:Pressed
    (Default|Scroll (Variables|Default|GetMainWidget) true)))

(event Input|MouseEvents|MouseWheelDown
  (params (Key :type Key%20Structure :default "None"))
  (:Pressed
    (Default|Scroll (Variables|Default|GetMainWidget) false)))

(event Input|KeyboardEvents|Tab
  (params (Key :type Key%20Structure :default "None"))
  (:Pressed
    (Default|ToggleChatMode (Variables|Default|GetMainWidget))))

(fn ConstructionScript)