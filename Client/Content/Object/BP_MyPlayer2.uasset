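; BP_MyPlayer2 is a player Blueprint that creates and owns the main HUD widget for the player's stats.
; BeginPlay creates a UI_Main widget, stores it as MainWidget and adds it to the viewport.
; When the SpawnPktReceived event fires, it pushes current and max HP, MP, and experience with the required amount into that widget.
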(event EventBeginPlay
  (bind _returnvalue (UserInterface|CreateWidget "/Game/Object/UI_Main.UI_Main_C"))
  (bind _output_get (Variables|Default|SetMainWidget _returnvalue))
  (UserInterface|Viewport|AddtoViewport _output_get 0))

(event Collision|EventActorBeginOverlap
  (params (OtherActor :type Actor%20Object%20Reference)))

(event EventTick
  (params (DeltaSeconds :type Float%20%28single-precision%29)))

(event EventSpawnPktReceived
  (bind _mainwidget (Variables|Default|GetMainWidget))
  (Default|SetHp _mainwidget (Variables|Default|GetHp) (Variables|Default|GetMaxHp))
  (Default|SetMp _mainwidget (Variables|Default|GetMp) (Variables|Default|GetMaxMp))
  (Default|SetExp _mainwidget (Variables|Default|GetExp) (Variables|Default|GetRequiredExp)))

(fn ConstructionScript)